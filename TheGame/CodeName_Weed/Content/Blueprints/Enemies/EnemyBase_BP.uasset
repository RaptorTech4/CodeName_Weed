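; Base enemy Blueprint that chases and attacks the player, with melee or ranged behavior selected by EnemyType.
; BeginPlay caches a PlayerBase_CBP reference, and Tick sets the blackboard "Chase?" key once the player is close, never clearing it here.
; Attack damages the player directly for melee, or plays a pumpkin montage and spawns a projectile from a socket.
; TakeDamage decrements Health, and a hit at zero or below triggers delayed destruction.
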(event Custom|Attack
  (bind _player (Variables|Default|GetPlayer))
  ;[1 1 1] Attacks
  (switch Utilities|FlowControl|Switch|SwitchonEnemyTypes_Enum (Variables|Default|GetEnemyType)
    (:NewEnumerator0
      (Utilities|IsValid _player
        (:Is%20Valid
          (Default|TakeDamige _player))))
    (:NewEnumerator1
      (Animation|PlayAnimMontage "/Game/Animations/Enemy/PumpkinHead/Pumpkin_Attacks.Pumpkin_Attacks" 1.0 "A2")
      (Utilities|FlowControl|Delay 0.5)
      (Game|SpawnActorfromClass "/Game/Blueprints/Enemies/PumkinProjectile_BP.PumkinProjectile_BP_C" (Transformation|GetWorldTransform (Variables|Default|GetProjectileSocket)) "Undefined" 0 0))))

(event Custom|TakeDamage
  ;[1 1 1] Health System
  (Math|Integer|CompareInt (Variables|Default|GetHealth)
    (:>
      (Math|Integer|DecrementInt (Variables|Default|GetHealth)
        (:%20%20
          (Animation|PlayAnimMontage "/Game/Animations/Enemy/PumpkinHead/Pumpkin_Attacks.Pumpkin_Attacks" 1.0 "H1"))))
    (:==
      (Variables|Default|SetIsDead? true :!label _label)
      (Utilities|FlowControl|Delay 3.0)
      (Actor|DestroyActor))
    (:<
      (goto _label))))

(event EventTick
  (params (DeltaSeconds :type Float%20%28single-precision%29))
  (bind _returnvalue (AI|GetBlackboard 0))
  (bind _player (Variables|Default|GetPlayer))
  ;[1 1 1] Overlap move to player
  (Utilities|IsValid _player
    (:Is%20Valid
      (Math|Float|CompareFloat (Transformation|GetDistanceTo _player self) 7e+02
        (:<
          (Utilities|IsValid _returnvalue
            (:Is%20Valid
              (AI|Components|Blackboard|SetValueasBool _returnvalue (Utilities|Name|MakeLiteralName "Chase?") true))))))))

(event EventBeginPlay
  ;[1 1 1] On Start
  (bind _outactors (Actor|GetAllActorsOfClass "/Game/Blueprints/Characters/PlayerBase_CBP.PlayerBase_CBP_C"))
  (for _array_element _outactors
    (Variables|Default|SetPlayer _array_element)
    (Variables|Default|SetIsDead? false)))

(fn ConstructionScript)
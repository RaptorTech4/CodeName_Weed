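; Camera actor that follows the player character, likely for a side-scrolling view.
; StartEvent stores the player reference, makes this actor the view target of the first player controller and sets a fixed rotation.
; Each tick it eases its location toward the player's with vector interpolation, giving a lagged follow while the rotation stays unchanged.
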(event Custom|StartEvent
  (params (Player_Ref :type Player%20Base%20CBP%20Object%20Reference))
  ;[1 1 1] Set view camera and set camera rotation
  (Variables|Default|SetPlayerBase_BP Player_Ref)
  (Game|Player|SetViewTargetwithBlend (Game|GetPlayerController 0) self 0.0 "VTBlend_Linear" 0.0 false)
  (Transformation|SetActorRotation "0,-90.000000, 0"))

(event EventTick
  (params (DeltaSeconds :type Float%20%28single-precision%29))
  ;[1 1 1] Camera states
  (Transformation|SetActorLocation (Math|Interpolation|VInterpTo (Transformation|GetActorLocation) (Transformation|GetActorLocation (Variables|Default|GetPlayerBase_BP)) (Utilities|Time|GetWorldDeltaSeconds) 2.5) false false))

(fn ConstructionScript)
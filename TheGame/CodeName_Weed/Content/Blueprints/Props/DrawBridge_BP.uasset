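; Drawbridge prop that swings the whole actor between a dropped pitch of -90 degrees and a raised pitch of zero.
; Drop and Up events each play their own timeline, with a Dropped flag that lets Up run only after a drop.
; Each update lerps from the current rotation toward the target pitch, keeping yaw and roll, so motion compounds rather than following the curve linearly.
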(event Custom|Drop
  (bind _returnvalue (Transformation|GetActorRotation))
  (Variables|Default|SetDropped? true)
  (bind _newtrack_0 (Timeline|Brd=idgeDown PlayFromStart)
    (:Update
      (Transformation|SetActorRelativeRotation (Math|Rotator|Lerp(Rotator) (Transformation|GetActorRotation) (Math|Rotator|MakeRotator (.roll _returnvalue) -9e+01 (.yaw _returnvalue)) _newtrack_0)))))

(event Custom|Up
  (bind _returnvalue (Transformation|GetActorRotation))
  (if (Variables|Default|GetDropped?)
    (Variables|Default|SetDropped? false)
    (bind _newtrack_0 (Timeline|BridgeUp PlayFromStart)
      (:Update
        (Transformation|SetActorRelativeRotation (Math|Rotator|Lerp(Rotator) (Transformation|GetActorRotation) (Math|Rotator|MakeRotator (.roll _returnvalue) 0.0 (.yaw _returnvalue)) _newtrack_0))))))

(fn ConstructionScript)
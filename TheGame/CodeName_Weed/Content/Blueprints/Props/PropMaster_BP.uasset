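; Master prop Blueprint that shifts between dream and nightmare states.
; Nightmare plays the TransformTime timeline and Dream reverses it, driving a named morph target on the skeletal mesh and a Colour scalar parameter.
; The Colour parameter lives on a dynamic material created from the mesh's first slot at BeginPlay.
; Static mesh hits from anything other than PlayerBase_CBP turn off skeletal mesh physics.
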(event OnComponentHit(StaticMesh)
  (params (HitComponent :type Primitive%20Component%20Object%20Reference) (OtherActor :type Actor%20Object%20Reference) (OtherComp :type Primitive%20Component%20Object%20Reference) (NormalImpulse :type Vector :default "0, 0, 0") (Hit :type Hit%20Result%20Structure%20%28by%20ref%29))
  ;[1 1 1] Pickup
  (Utilities|Casting|CastToPlayerBase_CBP OtherActor
    (:CastFailed
      (Physics|SetSimulatePhysics (Variables|Default|GetSkeletalMesh) false))))

(event Custom|Nightmare
  ;[1 1 1] Mothing
  (bind _transform (Timeline|TransformTime Play)
    (:Update
      (Components|SkeletalMesh|SetMorphTarget (Variables|Default|GetSkeletalMesh) (Variables|Default|GetName%20Of%20Morph) _transform false)
      (bind _output_get (Variables|Default|SetMMT _transform))
      (Rendering|Material|SetScalarParameterValue (Variables|Default|GetDynamicMaterial) "Colour" _output_get :!class /Script/Engine.MaterialInstanceDynamic))))

(event Custom|Dream
  ;[1 1 1] Mothing
  (bind _transform (Timeline|TransformTime Reverse)
    (:Update
      (Components|SkeletalMesh|SetMorphTarget (Variables|Default|GetSkeletalMesh) (Variables|Default|GetName%20Of%20Morph) _transform false)
      (bind _output_get (Variables|Default|SetMMT _transform))
      (Rendering|Material|SetScalarParameterValue (Variables|Default|GetDynamicMaterial) "Colour" _output_get :!class /Script/Engine.MaterialInstanceDynamic))))

(event EventBeginPlay
  (bind _skeletalmesh (Variables|Default|GetSkeletalMesh))
  ;[1 1 1] Mothing
  (bind _returnvalue (Rendering|Material|CreateDynamicMaterialInstance _skeletalmesh 0 (Rendering|Material|GetMaterial _skeletalmesh 0) :!class /Script/Engine.PrimitiveComponent))
  (bind _output_get (Variables|Default|SetDynamicMaterial _returnvalue)))

(fn ConstructionScript)
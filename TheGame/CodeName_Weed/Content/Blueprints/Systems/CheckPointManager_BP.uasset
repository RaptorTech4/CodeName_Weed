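; Checkpoint manager Blueprint that tracks the current checkpoint and its location.
; On BeginPlay it seeds the checkpoint location from PlayerBase_CBP actors in the level, keeping the last one found as the start position.
; UpdatedCurrentLocation receives a location and checkpoint, storing both when the checkpoint differs from the current one and leaving the location unchanged when it matches.
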(event Custom|UpdatedCurrentLocation
  (params (CurrentCheckpointLoc :type Vector) (CurrentCheckpoint :type Checkpoint%20BP%20Object%20Reference))
  ;[1 1 1] Get Checkpoint
  (if (== CurrentCheckpoint (Variables|Default|GetCurrentCheckpoint))
    (Variables|Default|SetCurrentCheckpoint CurrentCheckpoint)
    (else
      (Variables|Default|SetCurrentCheckpointLoc CurrentCheckpointLoc)
      (Variables|Default|SetCurrentCheckpoint CurrentCheckpoint))))

(event EventBeginPlay
  ;[1 1 1] Set Start Position Checkpoint
  (bind _outactors (Actor|GetAllActorsOfClass "/Game/Blueprints/Characters/PlayerBase_CBP.PlayerBase_CBP_C"))
  (for _array_element _outactors
    (Variables|Default|SetCurrentCheckpointLoc (Transformation|GetActorLocation _array_element))))

(fn ConstructionScript)
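; Checkpoint actor that registers itself as the current checkpoint when the player enters its radius.
; On BeginPlay it finds and caches the level's CheckPointManager_BP.
; Player overlap sends the checkpoint's location and self reference to that manager, then replays a timeline that spins the DreamCatcher mesh through a rotation lerp.
; Activation has no one-shot guard, so every re-entry updates the manager and restarts the spin.
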(event OnComponentBeginOverlap(Checkpointradius)
  (params (OverlappedComponent :type Primitive%20Component%20Object%20Reference) (OtherActor :type Actor%20Object%20Reference) (OtherComp :type Primitive%20Component%20Object%20Reference) (OtherBodyIndex :type Integer) (bFromSweep :type Boolean) (SweepResult :type Hit%20Result%20Structure%20%28by%20ref%29))
  ;[1 1 1] Updated to this checkpoint
  (Utilities|Casting|CastToPlayerBase_CBP OtherActor)
  (Utilities|IsValid (Variables|Default|GetCheckpointManager_BP)
    (:Is%20Valid
      (Default|UpdatedCurrentLocation (Variables|Default|GetCheckpointManager_BP) (Transformation|GetActorLocation) self)
      (bind _rotation_speed (Timeline|Activate%20Dreamcatcher%20animation PlayFromStart)
        (:Update
          (Transformation|SetWorldRotation (Variables|Default|GetDreamCatcher) (Math|Rotator|Lerp(Rotator) "0, 0, 0" "0,1080.000000, 0" _rotation_speed) false false))))))

(event EventBeginPlay
  ;[1 1 1] Get Checkpoint Manager
  (bind _outactors (Actor|GetAllActorsOfClass "/Game/Blueprints/Systems/CheckPointManager_BP.CheckPointManager_BP_C"))
  (for _array_element _outactors
    (Variables|Default|SetCheckpointManager_BP _array_element)))

(fn ConstructionScript)